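; Ghost text box actor that tracks whether Mia_PC is inside its collision component and whether Interact is held.
; Releasing Interact also clears the TownWidget exit text flag.
; The ghost dialogue is disconnected and never runs: a Ghostactive check and a one-shot cinematic typewriter widget that locks Mia's movement.
; Tick and the finished-writing event do nothing, so the live flags drive nothing in this graph.
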(event OnComponentEndOverlap(CollisionComponent)
  (params (OverlappedComponent :type Primitive%20Component%20Object%20Reference) (OtherActor :type Actor%20Object%20Reference) (OtherComp :type Primitive%20Component%20Object%20Reference) (OtherBodyIndex :type Integer))
  (Utilities|Casting|CastToMia_PC OtherActor)
  (Variables|Default|Setinside false))

(event OnComponentBeginOverlap(CollisionComponent)
  (params (OverlappedComponent :type Primitive%20Component%20Object%20Reference) (OtherActor :type Actor%20Object%20Reference) (OtherComp :type Primitive%20Component%20Object%20Reference) (OtherBodyIndex :type Integer) (bFromSweep :type Boolean) (SweepResult :type Hit%20Result%20Structure%20%28by%20ref%29))
  (Utilities|Casting|CastToMia_PC OtherActor)
  (Variables|Default|Setinside true))

(event Custom|FinishedWriting_Event_1)

(event EventBeginPlay)

(event Collision|EventActorBeginOverlap
  (params (OtherActor :type Actor%20Object%20Reference)))

(event EventTick
  (params (DeltaSeconds :type Float%20%28single-precision%29))
  (Utilities|FlowControl|Sequence))

(event Input|ActionEvents|InputActionInteract
  (params (Key :type Key%20Structure :default "None"))
  (:Pressed
    (Variables|Default|SetInteract true))
  (:Released
    (Variables|Default|SetInteract false)
    (Variables|/Game/Widgets/TextWidget.TextWidget_C|SetExitText (Variables|Default|GetTownWidget) false)))

(fn ConstructionScript)