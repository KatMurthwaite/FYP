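; A blocking trigger actor that stops the player from entering town with a dialogue from Mia about unpacking.
; On overlap it pauses the game and shows a NoIntoTown widget filled with her text, name and portrait.
; Tick unpauses the game while the Interact input is held.
; The widget is never removed here, and overlap does not filter by actor.
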(event EventBeginPlay)

(event Collision|EventActorBeginOverlap
  (params (OtherActor :type Actor%20Object%20Reference))
  (Game|SetGamePaused true)
  (bind _returnvalue (UserInterface|CreateWidget "/Game/Widgets/NoIntoTown.NoIntoTown_C"))
  (bind _output_get (Variables|Default|SetTownWidget _returnvalue))
  (UserInterface|Viewport|AddtoViewport _output_get 0)
  (Variables|/Game/Widgets/NoIntoTown.NoIntoTown_C|SetText%20box (Variables|Default|GetTownWidget) (Utilities|Text|MakeLiteralText "I don't feel like going into town right now... I still have a lot of unpacking to do"))
  (Variables|/Game/Widgets/NoIntoTown.NoIntoTown_C|SetName (Variables|Default|GetTownWidget) (Utilities|Text|MakeLiteralText "Mia"))
  (Variables|/Game/Widgets/NoIntoTown.NoIntoTown_C|SetImage (Variables|Default|GetTownWidget) (Variables|Default|GetMia_Normal)))

(event EventTick
  (params (DeltaSeconds :type Float%20%28single-precision%29))
  (if (Game|IsGamePaused)
    (if (Variables|Default|GetInteract)
      (Game|SetGamePaused false))))

(event Input|ActionEvents|InputActionInteract
  (params (Key :type Key%20Structure :default "None"))
  (:Pressed
    (Variables|Default|SetInteract true))
  (:Released
    (Variables|Default|SetInteract false)))

(fn ConstructionScript)