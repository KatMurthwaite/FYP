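; Tutorial bedtime trigger that tracks whether Mia is at the sleep spot once the boxes task is complete.
; Collision overlaps check the BoxesComplete flag in KatsInstance, then set BedTime true on entry and false on exit, each only once.
; Tick watches a text widget to add a fade-in when its text finishes, but the goodnight dialogue code that creates that widget is disconnected, so the fade stays inactive.
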(event OnComponentBeginOverlap(CollisionComponent)
  (params (OverlappedComponent :type Primitive%20Component%20Object%20Reference) (OtherActor :type Actor%20Object%20Reference) (OtherComp :type Primitive%20Component%20Object%20Reference) (OtherBodyIndex :type Integer) (bFromSweep :type Boolean) (SweepResult :type Hit%20Result%20Structure%20%28by%20ref%29))
  (Utilities|Casting|CastToMia_PC OtherActor)
  (bind _askats_instance (Utilities|Casting|CastToKatsInstance (Game|GetGameInstance)))
  (if (Variables|/Game/Blueprints/Variables/KatsInstance.KatsInstance_C|GetBoxesComplete _askats_instance)
    (Utilities|FlowControl|DoOnce false
      (:Completed
        (Variables|Default|SetBedTime true)))))

(event OnComponentEndOverlap(CollisionComponent)
  (params (OverlappedComponent :type Primitive%20Component%20Object%20Reference) (OtherActor :type Actor%20Object%20Reference) (OtherComp :type Primitive%20Component%20Object%20Reference) (OtherBodyIndex :type Integer))
  (Utilities|Casting|CastToMia_PC OtherActor)
  (bind _askats_instance (Utilities|Casting|CastToKatsInstance (Game|GetGameInstance)))
  (if (Variables|/Game/Blueprints/Variables/KatsInstance.KatsInstance_C|GetBoxesComplete _askats_instance)
    (Utilities|FlowControl|DoOnce false
      (:Completed
        (Variables|Default|SetBedTime false)))))

(event Custom|FinishedWriting_Event_0)

(event EventBeginPlay)

(event Collision|EventActorBeginOverlap
  (params (OtherActor :type Actor%20Object%20Reference)))

(event EventTick
  (params (DeltaSeconds :type Float%20%28single-precision%29))
  (bind _newvar_0 (Variables|Default|GetNewVar_0))
  (Utilities|IsValid _newvar_0
    (:Is%20Valid
      (if true
        (Utilities|FlowControl|DoOnce false
          (:Completed
            (if (Variables|/Game/Widgets/TextWidget_cinematic.TextWidget_cinematic_C|GetTextDone _newvar_0)
              (bind _returnvalue (UserInterface|CreateWidget "/Game/Widgets/fade-in.fade-in_C" (Game|GetPlayerController 0)))
              (UserInterface|Viewport|AddtoViewport _returnvalue 0)
              (Utilities|FlowControl|Delay 0.2))))))))

(fn ConstructionScript)