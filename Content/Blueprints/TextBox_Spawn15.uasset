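; TextBox_Spawn15 is an overlap-triggered dialogue actor that shows Mia reacting, once, to a door that was unlocked a second ago.
; It sets NoMove on Mia and spawns a TextWidget_cinematic using the GameInstance's text speed.
; The bound FinishedWriting handler is empty, so nothing here restores movement.
; Interact input only sets a flag and clears TownWidget.ExitText on release; an unreachable branch holds alternate flowers-and-dolls dialogue.
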(event Custom|FinishedWriting_Event_0)

(event Custom|FinishedWriting_Event_1)

(event EventBeginPlay)

(event Collision|EventActorBeginOverlap
  (params (OtherActor :type Actor%20Object%20Reference))
  (bind _askats_instance (Utilities|Casting|CastToKatsInstance (Game|GetGameInstance)))
  (Utilities|FlowControl|DoOnce false
    (:Completed
      (bind _asmia_pc (Utilities|Casting|CastToMia_PC (Game|GetPlayerCharacter 0)))
      (Variables|/Game/PlayerCharacter/Mia_PC.Mia_PC_C|SetNoMove _asmia_pc true)
      (bind _returnvalue (UserInterface|CreateWidget "/Game/Widgets/TextWidget_cinematic.TextWidget_cinematic_C" 0 "Mia" (Variables|Default|GetMia_Normal) (Variables|/Game/Blueprints/Variables/KatsInstance.KatsInstance_C|GetGameTextSpeed _askats_instance) (Utilities|Array|MakeArray "What the..." "This door was unlocked a second ago")))
      (bind _output_get (Variables|Default|SetNewVar_1 _returnvalue))
      (UserInterface|Viewport|AddtoViewport _output_get 0)
      (EventDispatchers|AssignFinishedWriting _output_get (delegate Custom|FinishedWriting_Event_0)))))

(event EventTick
  (params (DeltaSeconds :type Float%20%28single-precision%29))
  (Utilities|FlowControl|Sequence))

(event Input|ActionEvents|InputActionInteract
  (params (Key :type Key%20Structure))
  (:Pressed
    (Variables|Default|SetInteract true))
  (:Released
    (Variables|Default|SetInteract false)
    (Variables|/Game/Widgets/TextWidget.TextWidget_C|SetExitText (Variables|Default|GetTownWidget) false)))

(fn ConstructionScript)