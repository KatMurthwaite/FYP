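; Interactable actor named Food_Bakery that shows Mia's dialogue about creepy dolls.
; Pressing Interact locks the player's movement and opens a cinematic text widget, paced by the game instance's text speed.
; Box1 overlaps track Mia in an Inside flag, but the Interact branch is hard-wired true and ignores it.
; The finished-writing callback is empty, so this Blueprint never restores movement itself.
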(event OnComponentBeginOverlap(Box1)
  (params (OverlappedComponent :type Primitive%20Component%20Object%20Reference) (OtherActor :type Actor%20Object%20Reference) (OtherComp :type Primitive%20Component%20Object%20Reference) (OtherBodyIndex :type Integer) (bFromSweep :type Boolean) (SweepResult :type Hit%20Result%20Structure%20%28by%20ref%29))
  (Utilities|Casting|CastToMia_PC OtherActor)
  (Variables|Default|Setinside true))

(event OnComponentEndOverlap(Box1)
  (params (OverlappedComponent :type Primitive%20Component%20Object%20Reference) (OtherActor :type Actor%20Object%20Reference) (OtherComp :type Primitive%20Component%20Object%20Reference) (OtherBodyIndex :type Integer))
  (Utilities|Casting|CastToMia_PC OtherActor)
  (Variables|Default|Setinside false))

(event Custom|FinishedWriting_Event_0)

(event EventBeginPlay)

(event Collision|EventActorBeginOverlap
  (params (OtherActor :type Actor%20Object%20Reference)))

(event EventTick
  (params (DeltaSeconds :type Float%20%28single-precision%29)))

(event Input|ActionEvents|InputActionInteract
  (params (Key :type Key%20Structure :default "None"))
  (:Pressed
    (if true
      (bind _askats_instance (Utilities|Casting|CastToKatsInstance (Game|GetGameInstance)))
      (bind _asmia_pc (Utilities|Casting|CastToMia_PC (Game|GetPlayerCharacter 0)))
      (Variables|/Game/PlayerCharacter/Mia_PC.Mia_PC_C|SetNoMove _asmia_pc true)
      (bind _returnvalue (UserInterface|CreateWidget "/Game/Widgets/TextWidget_cinematic.TextWidget_cinematic_C" 0 "Mia" (Variables|Default|GetMia) (Variables|/Game/Blueprints/Variables/KatsInstance.KatsInstance_C|GetGameTextSpeed _askats_instance) (Utilities|Array|MakeArray "These dolls are creepy... Staring into my soul almost")))
      (bind _output_get (Variables|Default|SetNewVar_0 _returnvalue))
      (UserInterface|Viewport|AddtoViewport _output_get 0)
      (EventDispatchers|AssignFinishedWriting _output_get (delegate Custom|FinishedWriting_Event_0)))))

(fn ConstructionScript)