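; Trigger actor that stops Mia at the way to a school and shows her remark about it in a dialogue widget.
; On overlap it locks her movement and creates a TextWidget that types the line at the game instance's text speed, with her name and portrait.
; The finished-writing callback and Tick are empty, Interact only updates flags, and movement is never unlocked here.
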(event Custom|FinishedWriting_Event_0)

(event EventBeginPlay)

(event Collision|EventActorBeginOverlap
  (params (OtherActor :type Actor%20Object%20Reference))
  (bind _askats_instance (Utilities|Casting|CastToKatsInstance (Game|GetGameInstance)))
  (bind _asmia_pc (Utilities|Casting|CastToMia_PC OtherActor))
  (Variables|/Game/PlayerCharacter/Mia_PC.Mia_PC_C|SetNoMove _asmia_pc true)
  (bind _returnvalue (UserInterface|CreateWidget :Class "/Game/Widgets/TextWidget.TextWidget_C" :CharsPerSecond (Variables|/Game/Blueprints/Variables/KatsInstance.KatsInstance_C|GetGameTextSpeed _askats_instance)))
  (bind _output_get (Variables|Default|SetTownWidget _returnvalue))
  (UserInterface|Viewport|AddtoViewport _output_get 0)
  (Default|Write _output_get (Utilities|String|ToString(Text) (Utilities|Text|MakeLiteralText "This seems to lead to a school...")))
  (Variables|/Game/Widgets/TextWidget.TextWidget_C|SetName (Variables|Default|GetTownWidget) (Utilities|Text|MakeLiteralText "Mia"))
  (Variables|/Game/Widgets/TextWidget.TextWidget_C|SetImage (Variables|Default|GetTownWidget) (Variables|Default|GetMia_Normal))
  (EventDispatchers|AssignFinishedWriting _output_get (delegate Custom|FinishedWriting_Event_0)))

(event EventTick
  (params (DeltaSeconds :type Float%20%28single-precision%29))
  (Utilities|FlowControl|Sequence))

(event Input|ActionEvents|InputActionInteract
  (params (Key :type Key%20Structure :default "None"))
  (:Pressed
    (Variables|Default|SetInteract true))
  (:Released
    (Variables|Default|SetInteract false)
    (Variables|/Game/Widgets/TextWidget.TextWidget_C|SetExitText (Variables|Default|GetTownWidget) false)))

(fn ConstructionScript)