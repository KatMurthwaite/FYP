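; KatsInstance is a game instance Blueprint that manages save slots and music persisting across level transitions.
; On Init it loads Slot1 into SaveSlot1, or creates and saves a new KatsSaveGame without assigning that variable; Slot2 and Slot3 are only checked.
; SaveToSlot1 writes SaveSlot1 back to disk.
; Two music events spawn persistent, non-auto-destroyed 2D sounds for tutorial and town, storing their audio components.
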(event Custom|Music_Tutorial
  (params (NewParam :type Sound%20Base%20Object%20Reference))
  (bind _returnvalue (Audio|SpawnSound2D NewParam 1.0 1.0 (Variables|Default|GetStart%20Time) 0 true false))
  (Variables|Default|Setsound _returnvalue))

(event Custom|SaveToSlot1
  (SaveGame|SaveGametoSlot (Variables|Default|GetSave%20Slot%201) "Slot1"))

(event Custom|Music_IntoTown
  (params (NewParam :type Sound%20Base%20Object%20Reference))
  (bind _returnvalue (Audio|SpawnSound2D NewParam 1.0 1.0 0.0 0 true false))
  (Variables|Default|SetIntoTown _returnvalue))

(event EventInit
  (Utilities|FlowControl|Sequence
    (:then_0
      (bind _returnvalue (SaveGame|DoesSaveGameExist "Slot1"))
      (if _returnvalue
        (bind _returnvalue_2 (SaveGame|LoadGamefromSlot "Slot1"))
        (Variables|Default|SetSave%20Slot%201 _returnvalue_2)
        (Development|PrintString "Save slot 1 loaded")
        (else
          (bind _returnvalue_3 (SaveGame|CreateSaveGameObject "/Game/Blueprints/Variables/KatsSaveGame.KatsSaveGame_C"))
          (SaveGame|SaveGametoSlot _returnvalue_3 "Slot1")
          (Development|PrintString "Save slot 1 created"))))
    (:then_1
      (bind _returnvalue_4 (SaveGame|DoesSaveGameExist "Slot2"))
      (if _returnvalue_4
        _))
    (:then_2
      (bind _returnvalue_5 (SaveGame|DoesSaveGameExist "Slot3"))
      (if _returnvalue_5
        _))))